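; BP_TPSPlayer is the player Blueprint, carrying test hooks for enemy AI.
; Pressing the 1 key calls MakeNoise at the player's location with itself as instigator.
; Two unwired node chains get the AI controller of a BP_TP_EnemyBase and would set it to patrol, or to attack the player, but never run.
; The default events and construction script are empty.
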(event EventBeginPlay)

(event Collision|EventActorBeginOverlap
  (params (OtherActor :type Actor%20Object%20Reference)))

(event EventTick
  (params (DeltaSeconds :type Float%20%28single-precision%29)))

(event Input|KeyboardEvents|1
  (params (Key :type Key%20Structure :default "None"))
  (:Pressed
    (Class|Actor|MakeNoise 1.0 self (Transformation|GetActorLocation) 0.0 "None")))

(event Input|KeyboardEvents|2
  (params (Key :type Key%20Structure :default "None")))

(fn ConstructionScript)
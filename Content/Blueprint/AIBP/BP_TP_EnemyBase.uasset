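; Base enemy Blueprint that chases the first player character and attacks with a greatsword montage.
; ChasePlayer runs AI MoveTo, then on success calls Attack and re-calls itself after a short delay without awaiting the montage; a failed move ends the loop.
; Attack calls OnAttackEnd on montage completion, blend-out or interruption.
; Helper functions expose a patrol spline and map Idle, Walk and Sprint states to max walk speed.
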(event Custom|ChasePlayer
  (AI|AIMoveTo self "0, 0, 0" (Game|GetPlayerCharacter 0) 1e+02 false
    (:OnSuccess
      (CallFunction|Attack)
      (Utilities|FlowControl|Delay 0.05)
      (CallFunction|ChasePlayer))))

(event Custom|Attack
  (Animation|Montage|PlayMontage (Variables|Character|GetMesh) "/Game/MyResource/Animation/GreatSwordPack/greatswordattack_UE_Montage.greatswordattack_UE_Montage"
    (:OnCompleted
      _)
    (:OnBlendOut
      _)
    (:OnInterrupted
      _))
  (Default|CallOnAttackEnd))

(event EventBeginPlay)

(fn ConstructionScript)

(fn GetPatrolSpline
  (return (Variables|Default|GetPatrolSpline)))

(fn SetMovementSpeed
  (params (Speed :type E_MovementSpeed%20Enum :default "NewEnumerator0"))
  (bind _output_get (Variables|/Script/Engine.CharacterMovementComponent|SetMaxWalkSpeed (Variables|Character|GetCharacterMovement) (Utilities|Select :Index Speed :NewEnumerator0 0.0 :NewEnumerator1 3e+02 :NewEnumerator2 5e+02)))
  (return _output_get))